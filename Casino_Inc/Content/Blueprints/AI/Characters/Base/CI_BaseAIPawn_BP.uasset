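; Base AI pawn Blueprint that can request a path to a random destination through its path following component.
; GetRandomPath converts the pawn's XY location to 64-unit grid coordinates and passes it with a random end point in a fixed coordinate range to GetNewPath.
; BeginPlay and Tick only call the parent, and nothing in this Blueprint calls GetRandomPath.
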(event `self.ReceiveBeginPlay`
  (`parent.ReceiveBeginPlay`))

(event `self.ReceiveTick`
  (params (DeltaSeconds :type "Float (single-precision)"))
  (`parent.ReceiveTick` DeltaSeconds))

(fn `GetRandomPath`
  (`CI_PathFollowingComponent_CPP.GetNewPath` (`self.GetPathFollowingComponent`) (`KismetMathLibrary.MakeVector2D` (/ (.x (`self.K2_GetActorLocation`)) 64.0) (/ (.y (`self.K2_GetActorLocation`)) 64.0)) (`KismetMathLibrary.MakeVector2D` (`KismetMathLibrary.RandomFloatInRange` 0.0 99.0) (`KismetMathLibrary.RandomFloatInRange` 0.0 99.0))))

(fn `UserConstructionScript`)