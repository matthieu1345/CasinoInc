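; Game instance Blueprint that applies and updates global audio volume for the Master, Music, Effects and Voice sound classes.
; On Init, after a short delay, it activates the Mix_Global sound mix, loads the sound options if missing and applies the stored levels as class overrides.
; SetVolume clamps a new level, overrides the chosen class in the mix and writes it into SoundSaveOptions in memory.
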(event `self.ReceiveInit`
  (bind (_master _music _effects _voice) (break `SoundLevels` (`CI_SoundSaveGame_CPP.levels` (`self.soundSaveOptions`))))
  (`KismetSystemLibrary.Delay` 0.2)
  ;[1 1 1] Select sound mix
  (`GameplayStatics.SetBaseSoundMix` "/Game/Blueprints/Sound/Mix_Global.Mix_Global")
  (`GameplayStatics.PushSoundMixModifier` "/Game/Blueprints/Sound/Mix_Global.Mix_Global")
  (`self.soundSaveOptions`
    (:`then`
      _)
    (:`else`
      (`self.LoadSoundOptions`)))
  (`|ExecutionSequence`
    (:`then_0`
      (`GameplayStatics.SetSoundMixClassOverride` "/Game/Blueprints/Sound/Mix_Global.Mix_Global" "/Game/Blueprints/Sound/Master.Master" _master))
    (:`then_1`
      (`GameplayStatics.SetSoundMixClassOverride` "/Game/Blueprints/Sound/Mix_Global.Mix_Global" "/Game/Blueprints/Sound/Music.Music" _music))
    (:`then_2`
      (`GameplayStatics.SetSoundMixClassOverride` "/Game/Blueprints/Sound/Mix_Global.Mix_Global" "/Game/Blueprints/Sound/Effects.Effects" _effects))
    (:`then_3`
      (`GameplayStatics.SetSoundMixClassOverride` "/Game/Blueprints/Sound/Mix_Global.Mix_Global" "/Game/Blueprints/Sound/Voice.Voice" _voice))))

(fn `SetVolume`
  (params (Group :type "EVolumeGroup Enum" :default "VG_Master") (NewLevel :type "Float (double-precision)"))
  (bind _returnvalue (`KismetMathLibrary.FClamp` NewLevel))
  (bind _soundsaveoptions (`self.soundSaveOptions`))
  (bind _soundsaveoptions_2 (`self.soundSaveOptions`))
  (bind _soundsaveoptions_3 (`self.soundSaveOptions`))
  (bind _soundsaveoptions_4 (`self.soundSaveOptions`))
  (`self.soundSaveOptions`
    (:`then`
      _)
    (:`else`
      (`self.LoadSoundOptions`)))
  (switch `EVolumeGroup` Group
    (:`VG_Master`
      (`GameplayStatics.SetSoundMixClassOverride` "/Game/Blueprints/Sound/Mix_Global.Mix_Global" "/Game/Blueprints/Sound/Master.Master" _returnvalue)
      (bind _structout (setmembers `SoundLevels` :`StructRef` (`CI_SoundSaveGame_CPP.levels` _soundsaveoptions_2) :`master` _returnvalue))
      (set `CI_SoundSaveGame_CPP.levels` _structout _soundsaveoptions_2))
    (:`VG_Music`
      (`GameplayStatics.SetSoundMixClassOverride` "/Game/Blueprints/Sound/Mix_Global.Mix_Global" "/Game/Blueprints/Sound/Music.Music" _returnvalue)
      (bind _structout_2 (setmembers `SoundLevels` :`StructRef` (`CI_SoundSaveGame_CPP.levels` _soundsaveoptions_3) :`music` _returnvalue))
      (set `CI_SoundSaveGame_CPP.levels` _structout_2 _soundsaveoptions_3))
    (:`VG_Effects`
      (`GameplayStatics.SetSoundMixClassOverride` "/Game/Blueprints/Sound/Mix_Global.Mix_Global" "/Game/Blueprints/Sound/Effects.Effects" _returnvalue)
      (bind _structout_3 (setmembers `SoundLevels` :`StructRef` (`CI_SoundSaveGame_CPP.levels` _soundsaveoptions_4) :`effects` _returnvalue))
      (set `CI_SoundSaveGame_CPP.levels` _structout_3 _soundsaveoptions_4))
    (:`VG_Voice`
      (`GameplayStatics.SetSoundMixClassOverride` "/Game/Blueprints/Sound/Mix_Global.Mix_Global" "/Game/Blueprints/Sound/Voice.Voice" _returnvalue)
      (bind _structout_4 (setmembers `SoundLevels` :`StructRef` (`CI_SoundSaveGame_CPP.levels` _soundsaveoptions) :`voice` _returnvalue))
      (set `CI_SoundSaveGame_CPP.levels` _structout_4 _soundsaveoptions))))