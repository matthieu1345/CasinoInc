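; Tile map Blueprint that exposes events to create, destroy, reset and refresh a map of individual tiles.
; It calls CreateMap and DestroyMap, which are defined outside this graph, and makes the TilemapComponent editable on BeginPlay.
; Reset is gated by CheckDestroy, then recreates the map and applies DefaultMap.
; Other events print a destroy warning, manually update every tile's sprite, or fill the Ground layer with grass data.
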(event `DestroyMapBp`
  (`self.DestroyMap`))

(event `CreateMapBp`
  (`self.CreateMap`))

(event `self.DestroyWarning`
  (`KismetSystemLibrary.PrintString` "Are you sure you want to destroy the current map?" true true (struct :`R` 1.0 :`A` 1.0)))

(event `self.ReceiveBeginPlay`
  (`parent.ReceiveBeginPlay`)
  (`PaperTileMapComponent.MakeTileMapEditable` (`self.tilemapComponent`)))

(event `manualTick`
  (for _array_element (`self.allTiles`)
    (`CI_BaseTile_CPP.UpdateSprite` _array_element)))

(event `self.ReceiveTick`
  (params (DeltaSeconds :type "Float (single-precision)"))
  (`parent.ReceiveTick` DeltaSeconds))

(event `Make Editable`
  (`PaperTileMapComponent.MakeTileMapEditable` (`self.tilemapComponent`)))

(event `ResetMap`
  (bind _returnvalue (`self.CheckDestroy`))
  (if _returnvalue
    (`self.CreateMap`)
    (`PaperTileMapComponent.SetTileMap` (`self.tilemapComponent`) (`self.DefaultMap`))
    (`self.Make Editable`)))

(event `SetGroundTiles`
  (for _array_element (`CI_TileMapLayer_CPP.layerTiles` (`|GetArrayItem` (`self.allLayers`) (`KismetMathLibrary.Conv_ByteToInt` (enumliteral `ETileLayer` "TL_Ground"))))
    (set `CI_BaseTile_CPP.newTileDataComponent` "/Game/Blueprints/TileMap/Tiles/GrassData.GrassData_C" _array_element)
    (`CI_BaseTile_CPP.UpdateTileData` _array_element)))

(fn `UserConstructionScript`)